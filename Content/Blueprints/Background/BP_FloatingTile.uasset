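; BP_FloatingTile is a background actor that drifts vertically at a constant PatrolSpeed.
; BeginPlay randomly picks an up or down direction and a patrol time between MinTime and MaxTime.
; Tick moves the tile along Z without sweep and rerolls the patrol time whenever the timer exceeds it.
; The direction is never reversed after BeginPlay, so the rerolls do not affect the motion.
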(event `self.ReceiveBeginPlay`
  (set `self.PatrolTime` (`KismetMathLibrary.RandomFloatInRange` (`self.MinTime`) (`self.MaxTime`)))
  (if (<= (`KismetMathLibrary.RandomFloat`) 0.5)
    (set `self.ZDir` -1)
    (else
      (set `self.ZDir` 1))))

(event `self.ReceiveTick`
  (params (DeltaSeconds :type "Float (single-precision)"))
  (`self.K2_SetActorLocation` (+ (`self.K2_GetActorLocation`) (`KismetMathLibrary.MakeVector` 0.0 0.0 (* (* (`self.ZDir`) (`self.PatrolSpeed`)) DeltaSeconds))))
  (bind _output_get (set `self.Timer` (+ (`self.Timer`) DeltaSeconds)))
  (if (> _output_get (`self.PatrolTime`))
    (set `self.Timer` 0.0)
    (`self.RandomPatrolTime`)))

(fn `RandomPatrolTime`
  (set `self.PatrolTime` (`KismetMathLibrary.RandomFloatInRange` (`self.MinTime`) (`self.MaxTime`))))

(fn `UserConstructionScript`)