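; BP_ScrollingTile is a background tile actor that scrolls horizontally at a constant speed.
; On BeginPlay it picks a random direction sign and a random starting X between MinX and MaxX.
; Each Tick, MoveTile offsets it along X by direction, MoveSpeed and delta time; despite its name, ZDir drives X movement.
; No wrapping or bounds check limits the movement after the initial placement.
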(event `self.ReceiveBeginPlay`
  (`self.RandomDirection`)
  (`self.RandomPosX`))

(event `self.ReceiveTick`
  (params (DeltaSeconds :type "Float (single-precision)"))
  (`self.K2_SetActorLocation` (+ (`self.K2_GetActorLocation`) (`KismetMathLibrary.MakeVector` (* (* (`self.ZDir`) (`self.MoveSpeed`)) DeltaSeconds))))
  (if true
    _))

(fn `RandomDirection`
  (if (<= (`KismetMathLibrary.RandomFloat`) 0.5)
    (set `self.ZDir` -1)
    (else
      (set `self.ZDir` 1))))

(fn `RandomPosX`
  (bind (_returnvalue_x _returnvalue_y _returnvalue_z) (`KismetMathLibrary.BreakVector` (`self.K2_GetActorLocation`)))
  (`self.K2_SetActorLocation` (`KismetMathLibrary.MakeVector` (`KismetMathLibrary.RandomFloatInRange` (`self.MinX`) (`self.MaxX`)) _returnvalue_y _returnvalue_z)))

(fn `UserConstructionScript`)