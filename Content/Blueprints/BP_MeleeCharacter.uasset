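; Side-view melee fighter character that flips its mesh to match horizontal velocity and takes hits from other fighters.
; Capsule overlaps with "Hit"-tagged components apply the attacker's damage and facing-based knockback; blocking cuts damage only when facing right against a left-facing attacker.
; Helpers set attack data, animate post-process intensity and swap face textures, though FaceMaterial creation is disconnected.
; Limb collision toggles almost all target RightHandBox, including both leg functions.
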(event `self.ReceiveBeginPlay`)

(event `self.ReceiveTick`
  (params (DeltaSeconds :type "Float (single-precision)"))
  (bind _returnvalue_x (`KismetMathLibrary.BreakVector` (`self.GetVelocity`)))
  (bind _returnvalue_x_2 (`KismetMathLibrary.BreakVector` (`self.GetVelocity`)))
  (bind _mesh (`self.Mesh`))
  (bind _mesh_2 (`self.Mesh`))
  (bind (_relativescale3d_x _relativescale3d_y _relativescale3d_z) (`KismetMathLibrary.BreakVector` (`SceneComponent.RelativeScale3D` _mesh)))
  (bind (_relativerotation_roll _relativerotation_pitch _relativerotation_yaw) (`KismetMathLibrary.BreakRotator` (`SceneComponent.RelativeRotation` (`self.Mesh`))))
  (bind (_relativescale3d_x_2 _relativescale3d_y_2 _relativescale3d_z_2) (`KismetMathLibrary.BreakVector` (`SceneComponent.RelativeScale3D` _mesh_2)))
  (bind (_relativerotation_roll_2 _relativerotation_pitch_2 _relativerotation_yaw_2) (`KismetMathLibrary.BreakRotator` (`SceneComponent.RelativeRotation` (`self.Mesh`))))
  (if (and (`self.FacingLeft?`) (> _returnvalue_x_2 0.0))
    (`SceneComponent.K2_SetRelativeRotation` (`self.Mesh`) (`KismetMathLibrary.MakeRotator` 0.0 0.0 (- _relativerotation_yaw 180.0)) false false)
    (set `self.FacingLeft?` false)
    (`SceneComponent.SetRelativeScale3D` _mesh_2 (`KismetMathLibrary.MakeVector` 1.0 _relativescale3d_y_2 _relativescale3d_z_2))
    (elif (and (not (`self.FacingLeft?`)) (< _returnvalue_x 0.0))
      (`SceneComponent.K2_SetRelativeRotation` (`self.Mesh`) (`KismetMathLibrary.MakeRotator` 0.0 0.0 (+ _relativerotation_yaw_2 180.0)) false false)
      (set `self.FacingLeft?` true)
      (`SceneComponent.SetRelativeScale3D` _mesh (`KismetMathLibrary.MakeVector` -1.0 _relativescale3d_y _relativescale3d_z)))))

(event `self.CapsuleComponent.OnComponentBeginOverlap`
  (params (OverlappedComponent :type "PrimitiveComponent Object Reference") (OtherActor :type "Actor Object Reference") (OtherComp :type "PrimitiveComponent Object Reference") (OtherBodyIndex :type Integer) (bFromSweep :type Boolean) (SweepResult :type "HitResult Structure (by ref)"))
  (if (and (`ActorComponent.ComponentHasTag` OtherComp "Hit") (not (== OtherActor self)))
    (`|ExecutionSequence`
      (:`then_1`
        (bind _asbp_melee_character (cast `/Game/Blueprints/BP_MeleeCharacter` OtherActor))
        (if (`self.IsBlocking?`)
          (if (and (not (`self.FacingLeft?`)) (`/Game/Blueprints/BP_MeleeCharacter.FacingLeft?` _asbp_melee_character))
            (set `self.Health` (- (`self.Health`) (* (`/Game/Blueprints/BP_MeleeCharacter.AttackDamage` _asbp_melee_character) 0.2)))
            (else
              (bind (_knockbackvector_x _knockbackvector_y _knockbackvector_z) (`KismetMathLibrary.BreakVector` (`/Game/Blueprints/BP_MeleeCharacter.KnockbackVector` _asbp_melee_character)))
              (`CharacterMovementComponent.AddImpulse` (`self.CharacterMovement`) (`KismetMathLibrary.MakeVector` (* (select `bool` (`/Game/Blueprints/BP_MeleeCharacter.FacingLeft?` _asbp_melee_character) :`false` 1 :`true` -1) _knockbackvector_x) _knockbackvector_y _knockbackvector_z) true :!label _label)
              (set `self.Health` (- (`self.Health`) (`/Game/Blueprints/BP_MeleeCharacter.AttackDamage` _asbp_melee_character)))
              (set `self.IsDamaged?` true)))
          (else
            (goto _label)))))))

(event `PostProcessEffect`
  (bind (_direction _intensity) (`Timeline|Timeline_0`)
    (:`Update`
      (setmembers `PostProcessSettings` :`StructRef` (`PostProcessVolume.Settings` (`self.GlobalPPV`)) :`SceneFringeIntensity` _intensity))))

(fn `ChangeExpression`
  (params (ExpressionEnum :type "/Game/Data/Expressions Enum" :default "NewEnumerator0"))
  (locals (ArrayInt :type Integer))
  (bind _facematerial (`self.faceMaterial`))
  (switch `/Game/Data/Expressions` ExpressionEnum
    (:`NewEnumerator0`
      (`MaterialInstanceDynamic.SetTextureParameterValue` _facematerial "Sprite" "/Game/ArtAssets/RoboCharacter/face02.face02" :!label _label))
    (:`NewEnumerator1`
      (`MaterialInstanceDynamic.SetTextureParameterValue` _facematerial "Sprite" "/Game/ArtAssets/RoboCharacter/face03.face03"))
    (:`NewEnumerator2`
      (goto _label))
    (:`NewEnumerator3`
      (`MaterialInstanceDynamic.SetTextureParameterValue` _facematerial "Sprite" "/Game/ArtAssets/RoboCharacter/face04.face04"))
    (:`NewEnumerator4`
      (`MaterialInstanceDynamic.SetTextureParameterValue` _facematerial "Sprite" "/Game/ArtAssets/RoboCharacter/face01.face01"))))

(fn `EnableLeftHandCollision`
  (params (`Enable?` :type Boolean))
  (if `Enable?`
    (`PrimitiveComponent.SetCollisionEnabled` (`self.LeftHandBox`) "QueryAndPhysics")
    (else
      (`PrimitiveComponent.SetCollisionEnabled` (`self.RightHandBox`) "NoCollision"))))

(fn `EnableLeftLegCollision`
  (params (`Enable?` :type Boolean))
  (if `Enable?`
    (`PrimitiveComponent.SetCollisionEnabled` (`self.RightHandBox`) "QueryAndPhysics")
    (else
      (`PrimitiveComponent.SetCollisionEnabled` (`self.RightHandBox`) "NoCollision"))))

(fn `EnableRightHandCollision`
  (params (`Enable?` :type Boolean))
  (if `Enable?`
    (`PrimitiveComponent.SetCollisionEnabled` (`self.RightHandBox`) "QueryAndPhysics")
    (else
      (`PrimitiveComponent.SetCollisionEnabled` (`self.RightHandBox`) "NoCollision"))))

(fn `EnableRightLegCollision`
  (params (`Enable?` :type Boolean))
  (if `Enable?`
    (`PrimitiveComponent.SetCollisionEnabled` (`self.RightHandBox`) "QueryAndPhysics")
    (else
      (`PrimitiveComponent.SetCollisionEnabled` (`self.RightHandBox`) "NoCollision"))))

(fn `FaceToLeft`
  (params (`FaceLeft?` :type Boolean))
  (bind _mesh (`self.Mesh`))
  (bind _mesh_2 (`self.Mesh`))
  (bind (_relativescale3d_x _relativescale3d_y _relativescale3d_z) (`KismetMathLibrary.BreakVector` (`SceneComponent.RelativeScale3D` _mesh)))
  (bind (_relativescale3d_x_2 _relativescale3d_y_2 _relativescale3d_z_2) (`KismetMathLibrary.BreakVector` (`SceneComponent.RelativeScale3D` _mesh_2)))
  (bind _output_get (set `self.FacingLeft?` `FaceLeft?`))
  (if _output_get
    (`SceneComponent.SetRelativeScale3D` _mesh_2 (`KismetMathLibrary.MakeVector` -1.0 _relativescale3d_y_2 _relativescale3d_z_2))
    (else
      (`SceneComponent.SetRelativeScale3D` _mesh (`KismetMathLibrary.MakeVector` 1.0 _relativescale3d_y _relativescale3d_z)))))

(fn `LoadData`
  (bind _returnvalue (`GameplayStatics.LoadGameFromSlot` "ImageData"))
  (bind _assave_image_data (cast `/Game/Blueprints/Save_ImageData` _returnvalue))
  (set `self.ExpressionData` (`/Game/Blueprints/Save_ImageData.ImageData` _assave_image_data)))

(fn `UpdateHitData`
  (params (Knockback :type "Vector Structure") (Damage :type "Float (double-precision)"))
  (set `self.KnockbackVector` Knockback)
  (set `self.AttackDamage` Damage))

(fn `UserConstructionScript`)