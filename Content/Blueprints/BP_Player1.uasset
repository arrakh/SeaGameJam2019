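; BP_Player1 is the player one character, with side-to-side movement, jumping, punching and kicking.
; Its own set of "_1" input bindings drives movement along the world X axis and the built-in Jump and StopJumping.
; Punch and kick presses are passed straight to CharAnimInstance through PunchAnim and KickAnim, with no hit or damage logic in this graph.
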(event `InputAxis|MoveHorizontal_1`
  (params (AxisValue :type "Float (single-precision)"))
  (`self.AddMovementInput` (1.0 0.0 0.0) AxisValue))

(event `InputAction|Jump_2` :consume false
  (params (Key :type "Key Structure")))

(event `InputAction|Jump_1`
  (params (Key :type "Key Structure"))
  (:`Pressed`
    (`self.Jump`))
  (:`Released`
    (`self.StopJumping`)))

(event `InputAction|Kick_2` :consume false
  (params (Key :type "Key Structure")))

(event `InputAction|Punch_2` :consume false
  (params (Key :type "Key Structure")))

(event `InputAction|Punch_1`
  (params (Key :type "Key Structure"))
  (:`Pressed`
    (`/Game/Blueprints/AnimBP_Boy.PunchAnim` (`self.CharAnimInstance`))))

(event `InputAction|Block_2` :consume false
  (params (Key :type "Key Structure")))

(event `InputAction|Kick_1`
  (params (Key :type "Key Structure"))
  (:`Pressed`
    (`/Game/Blueprints/AnimBP_Boy.KickAnim` (`self.CharAnimInstance`))))

(event `InputAction|Block_1` :consume false
  (params (Key :type "Key Structure")))

(fn `UserConstructionScript`
  (`parent.UserConstructionScript`))