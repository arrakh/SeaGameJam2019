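; Robot fighter Blueprint that supplies the hit boxes for punches and kicks.
; It overrides four enable events to toggle collision on its hand and leg boxes, using query-only except the right leg, which also enables physics.
; The construction script creates a dynamic material from the robot's decal and stores it as FaceMaterial.
; Tick only calls the parent, and BeginPlay is disabled.
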(event `self.ReceiveTick`
  (params (DeltaSeconds :type "Float (single-precision)"))
  (`parent.ReceiveTick` DeltaSeconds))

(event `self.EnableLeftHandCollision`
  (params (`Enable?` :type Boolean))
  (bind _lefthandbox_robot (`self.LeftHandBox_Robot`))
  ;[1 1 1] Overriden collision function for punch and kick
  (if `Enable?`
    (`PrimitiveComponent.SetCollisionEnabled` _lefthandbox_robot "QueryOnly")
    (else
      (`PrimitiveComponent.SetCollisionEnabled` _lefthandbox_robot "NoCollision"))))

(event `self.EnableLeftLegCollision`
  (params (`Enable?` :type Boolean))
  (bind _leftlegbox_robot (`self.LeftLegBox_Robot`))
  ;[1 1 1] Overriden collision function for punch and kick
  (if `Enable?`
    (`PrimitiveComponent.SetCollisionEnabled` _leftlegbox_robot "QueryOnly")
    (else
      (`PrimitiveComponent.SetCollisionEnabled` _leftlegbox_robot "NoCollision"))))

(event `self.EnableRightHandCollision`
  (params (`Enable?` :type Boolean))
  (bind _righthandbox_robot (`self.RightHandBox_Robot`))
  ;[1 1 1] Overriden collision function for punch and kick
  (if `Enable?`
    (`PrimitiveComponent.SetCollisionEnabled` _righthandbox_robot "QueryOnly")
    (else
      (`PrimitiveComponent.SetCollisionEnabled` _righthandbox_robot "NoCollision"))))

(event `self.EnableRightLegCollision`
  (params (`Enable?` :type Boolean))
  (bind _rightlegbox_robot (`self.RightLegBox_Robot`))
  ;[1 1 1] Overriden collision function for punch and kick
  (if `Enable?`
    (`PrimitiveComponent.SetCollisionEnabled` _rightlegbox_robot "QueryAndPhysics")
    (else
      (`PrimitiveComponent.SetCollisionEnabled` _rightlegbox_robot "NoCollision"))))

(fn `UserConstructionScript`
  (bind _returnvalue (`DecalComponent.CreateDynamicMaterialInstance` (`self.Decal_Robot`)))
  (set `self.faceMaterial` _returnvalue))