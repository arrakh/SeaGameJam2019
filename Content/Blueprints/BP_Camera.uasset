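; BP_Camera is a shared side-view camera that follows and frames every BP_MeleeCharacter.
; It gathers the characters once shortly after BeginPlay, then a fast looping timer records their X and Z positions.
; The extremes set the root's location on the Y=0 plane, slightly lowered, and the clamped spring arm length for zoom.
; Span uses summed absolute extremes, so centering assumes characters straddle zero on each axis.
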(event `self.ReceiveActorBeginOverlap`
  (params (OtherActor :type "Actor Object Reference")))

(event `self.ReceiveBeginPlay`
  (`KismetSystemLibrary.Delay` 0.1)
  (bind _outactors (`GameplayStatics.GetAllActorsOfClass` "/Game/Blueprints/BP_MeleeCharacter.BP_MeleeCharacter_C"))
  (set `self.Follow` _outactors)
  (`KismetSystemLibrary.K2_SetTimerDelegate` (delegate `SetPos`) 0.01 true))

(event `SetPos`
  (bind _xpos (`self.XPos`))
  (bind _zpos (`self.ZPos`))
  (bind (_indexofminvalue _minvalue) (`KismetMathLibrary.MinOfFloatArray` _xpos))
  (bind (_indexofminvalue_2 _minvalue_2) (`KismetMathLibrary.MinOfFloatArray` _zpos))
  (bind _returnvalue (+ (`KismetMathLibrary.Abs` _minvalue_2) (`KismetMathLibrary.Abs` (`.MaxValue` (`KismetMathLibrary.MaxOfFloatArray` _zpos)))))
  (bind _returnvalue_2 (+ (`KismetMathLibrary.Abs` _minvalue) (`KismetMathLibrary.Abs` (`.MaxValue` (`KismetMathLibrary.MaxOfFloatArray` _xpos)))))
  (`|ExecutionSequence`
    (:`then_0`
      (for (_array_element _array_index) (`self.Follow`)
        (bind (_returnvalue_x _returnvalue_y _returnvalue_z) (`KismetMathLibrary.BreakVector` (`self.K2_GetActorLocation` _array_element)))
        (`KismetArrayLibrary.Array_Set` (`self.XPos`) _array_index _returnvalue_x true)
        (`KismetArrayLibrary.Array_Set` (`self.ZPos`) _array_index _returnvalue_z true))
      (bind _output_get (set `self.FollowLoc` (`KismetMathLibrary.MakeVector` (+ (/ _returnvalue_2 2.0) _minvalue) 0.0 (+ (/ _returnvalue 2.0) _minvalue_2 -40.0))))
      (`SceneComponent.K2_SetWorldLocation` (`self.DefaultSceneRoot`) _output_get false false)
      (set `SpringArmComponent.TargetArmLength` (`KismetMathLibrary.FClamp` (/ (+ _returnvalue_2 _returnvalue) 1.8) 50.0 2000.0) (`self.SpringArm`)))))

(fn `UserConstructionScript`)