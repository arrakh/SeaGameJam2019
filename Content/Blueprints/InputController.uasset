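; Input hub that drives two BP_MeleeCharacter fighters from separate per-player input mappings.
; At BeginPlay it finds the characters in the level, filling Player1 first if empty and otherwise Player2, so assignment follows search order.
; Horizontal axes add movement along world X, while jump, punch and kick presses set start flags on the matching character and jump release calls StopJumping.
; An obsolete SetActorLocation movement snippet remains unconnected.
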(event `self.ReceiveBeginPlay`
  (bind _outactors (`GameplayStatics.GetAllActorsOfClass` "/Game/Blueprints/BP_MeleeCharacter.BP_MeleeCharacter_C"))
  (for _array_element _outactors
    (if (== (`self.Player1`) null)
      (set `self.Player1` _array_element)
      (else
        (set `self.Player2` _array_element)))))

(event `InputAxis|MoveHorizontal_1`
  (params (AxisValue :type "Float (single-precision)"))
  ;[1 1 1] Player 1
  (`self.AddMovementInput` (`self.Player1`) (1.0 0.0 0.0) AxisValue false))

(event `InputAxis|MoveHorizontal_2`
  (params (AxisValue :type "Float (single-precision)"))
  ;[1 1 1] Player  2
  (`self.AddMovementInput` (`self.Player2`) (1.0 0.0 0.0) AxisValue false))

(event `InputAction|Jump_2`
  (params (Key :type "Key Structure"))
  (bind _player2 (`self.Player2`))
  ;[1 1 1] Player  2
  (:`Pressed`
    (set `/Game/Blueprints/BP_MeleeCharacter.StartJump?` true _player2))
  (:`Released`
    (`Character.StopJumping` _player2)))

(event `InputAction|Jump_1`
  (params (Key :type "Key Structure"))
  (bind _player1 (`self.Player1`))
  ;[1 1 1] Player 1
  (:`Pressed`
    (set `/Game/Blueprints/BP_MeleeCharacter.StartJump?` true _player1))
  (:`Released`
    (`Character.StopJumping` _player1)))

(event `InputAction|Kick_2`
  (params (Key :type "Key Structure"))
  ;[1 1 1] Player  2
  (:`Pressed`
    (set `/Game/Blueprints/BP_MeleeCharacter.StartKick?` true (`self.Player2`))))

(event `InputAction|Punch_1`
  (params (Key :type "Key Structure"))
  ;[1 1 1] Player 1
  (:`Pressed`
    (set `/Game/Blueprints/BP_MeleeCharacter.StartPunch?` true (`self.Player1`))))

(event `InputAction|Punch_2`
  (params (Key :type "Key Structure"))
  ;[1 1 1] Player  2
  (:`Pressed`
    (set `/Game/Blueprints/BP_MeleeCharacter.StartPunch?` true (`self.Player2`))))

(event `InputAction|Block_2`
  (params (Key :type "Key Structure"))
  ;[1 1 1] Player  2
)

(event `InputAction|Kick_1`
  (params (Key :type "Key Structure"))
  ;[1 1 1] Player 1
  (:`Pressed`
    (set `/Game/Blueprints/BP_MeleeCharacter.StartKick?` true (`self.Player1`))))

(event `InputAction|Block_1`
  (params (Key :type "Key Structure"))
  ;[1 1 1] Player 1
)

(fn `UserConstructionScript`)